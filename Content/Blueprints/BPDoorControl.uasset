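; BPDoorControl is a door control that triggers a target door on a button click and reports that door's state to JavaScript.
; The received button-click event calls TriggerDoors on TargetDoor.
; The construction script binds to TargetDoor's state-change event.
; Each state change creates a NotifyDoorState JavaScript call object, fills in the new state and invokes it on the control's JavaScript call context.
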(event Custom|Received_ButtonClicked
  (Default|TriggerDoors (Variables|Default|GetTargetDoor)))

(fn ConstructionScript
  (|CallParentFunction)
  (EventDispatchers|BindEventtoDoorStateChanged (Variables|Default|GetTargetDoor) (EventDispatchers|CreateEvent self :!event OnDoorStateChanged)))

(fn OnDoorStateChanged
  (params (NewDoorState :type EDoorState%20Enum :default "NewEnumerator0"))
  (bind _asjscall_doorcontrol_notifydoorstate_c (Utilities|Casting|CastToJSCall_DoorControl_NotifyDoorState (Class|RadiantJavaScriptFunctionCallLibrary|NewJavaScriptFunctionCallInstance "/Game/Blueprints/JSCall_DoorControl_NotifyDoorState.JSCall_DoorControl_NotifyDoorState_C")))
  (Variables|/Game/Blueprints/JSCall_DoorControl_NotifyDoorState.JSCall_DoorControl_NotifyDoorState_C|SetDoorState _asjscall_doorcontrol_notifydoorstate_c NewDoorState)
  (Class|RadiantJavaScriptFunctionCall|Invoke _asjscall_doorcontrol_notifydoorstate_c (Class|RadiantWebViewActor|GetJavaScriptCallContext)))